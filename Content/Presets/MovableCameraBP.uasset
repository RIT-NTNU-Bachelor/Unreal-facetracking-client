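; MovableCameraBP is a camera Blueprint that cycles through presets from the CameraPresets data table with the N key.
; Releasing N increments CurrentIndex, wraps it to zero past the table's row count, and passes it to ChangeCameraSettings, which is defined outside these graphs.
; BeginPlay and pressing N both print a "Hello" debug string, and the construction script is empty.
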(event `self.ReceiveBeginPlay`
  (`KismetSystemLibrary.PrintString` "Hello" :!label _label))

(event `Key|N` :paused true
  (params (Key :type "Key Structure"))
  (bind _currentindex (`self.CurrentIndex`))
  (:`Pressed`
    (goto _label))
  (:`Released`
    (bind _result (`/Engine/EditorBlueprintResources/StandardMacros.IncrementInt` (`self.CurrentIndex`))
      (:`  `
        (set `self.CurrentIndex` _result)
        (bind _outrownames (`DataTableFunctionLibrary.GetDataTableRowNames` "/Game/Presets/CameraPresets.CameraPresets"))
        (if (>= _currentindex (`KismetArrayLibrary.Array_Length` _outrownames))
          (bind _output_get (set `self.CurrentIndex` 0))
          (`self.ChangeCameraSettings` _output_get)
          (else
            (`self.ChangeCameraSettings` _currentindex)))))))

(fn `UserConstructionScript`)